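; TrashChuteBP is a chute that continually spawns trash actors at its Scene component's location.
; A looping timer started on BeginPlay fires SpawnStuff every fraction of a second, spawning a random class from the TireFrame array.
; When the possessed PlayerBP's ChangeCube counter equals its threshold, the chute resets it and spawns a ClearBP instead.
; Spawns ignore collisions, and the timer only starts if the cast to PlayerBP succeeds.
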(event `self.ReceiveBeginPlay`
  (bind _asplayer_bp (cast `/Game/Blueprints/PlayerBP` (`Controller.K2_GetPawn` (`GameplayStatics.GetPlayerController` 0))))
  (set `self.PlayerBP` _asplayer_bp)
  (`KismetSystemLibrary.K2_SetTimerDelegate` (delegate `SpawnStuff`) 0.7 true))

(event `SpawnStuff`
  (bind _tireframe (`self.TireFrame`))
  (bind _returnvalue_location (`KismetMathLibrary.BreakTransform` (`SceneComponent.K2_GetComponentToWorld` (`self.Scene`))))
  (bind _returnvalue_location_2 (`KismetMathLibrary.BreakTransform` (`SceneComponent.K2_GetComponentToWorld` (`self.Scene`))))
  (if (== (`/Game/Blueprints/PlayerBP.ChangeCube` (`self.PlayerBP`)) 25)
    (set `/Game/Blueprints/PlayerBP.ChangeCube` 0 (`self.PlayerBP`))
    (`|SpawnActorFromClass` "/Game/Blueprints/ClearBP.ClearBP_C" (`KismetMathLibrary.MakeTransform` _returnvalue_location (struct :`Roll` 10.0)) "AlwaysSpawn" "OverrideRootScale" null null)
    (else
      (`|SpawnActorFromClass` (`|GetArrayItem` _tireframe (`KismetMathLibrary.RandomInteger` (`KismetArrayLibrary.Array_Length` _tireframe))) (`KismetMathLibrary.MakeTransform` _returnvalue_location_2 (struct :`Yaw` 10.0 :`Roll` 10.0)) "AlwaysSpawn" "OverrideRootScale" null null))))

(fn `UserConstructionScript`)