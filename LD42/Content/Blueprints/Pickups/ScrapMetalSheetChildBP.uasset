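; Scrap metal sheet pickup, a child Blueprint of a parent pickup class.
; On BeginPlay it applies a fixed local rotation offset to the actor.
; The first hit on its PickupObject component plays a metal dropping sound at the impact point, with a boolean flag preventing repeats.
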(event `self.ReceiveBeginPlay`
  (`self.K2_AddActorLocalRotation` (struct :`Yaw` 10.0 :`Roll` 90.0)))

(event `self.PickupObject.OnComponentHit`
  (params (HitComponent :type "PrimitiveComponent Object Reference") (OtherActor :type "Actor Object Reference") (OtherComp :type "PrimitiveComponent Object Reference") (NormalImpulse :type "Vector Structure") (Hit :type "HitResult Structure (by ref)"))
  (if (not (`self.NewVar_0`))
    (`GameplayStatics.PlaySoundAtLocation` "/Game/metaldropping2.metaldropping2" (`.ImpactPoint` (`GameplayStatics.BreakHitResult` Hit)))
    (set `self.NewVar_0` true)))

(fn `UserConstructionScript`
  (`parent.UserConstructionScript`))