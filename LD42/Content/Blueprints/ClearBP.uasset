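; ClearBP is a one-shot powerup actor that clears scrap from the level.
; Tick polls the ActivatePowerup flag, resets it when set and calls DeleteScrap.
; DeleteScrap finds every actor of each class in the RemoveTrash array, destroys them all, then destroys itself.
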(event `self.ReceiveTick`
  (params (DeltaSeconds :type "Float (single-precision)"))
  (if (`self.ActivatePowerup`)
    (set `self.ActivatePowerup` false)
    (`self.DeleteScrap`)))

(event `DeleteScrap`
  (for _array_element (`self.RemoveTrash`)
    (bind _outactors (`GameplayStatics.GetAllActorsOfClass` _array_element))
    (for _array_element_2 _outactors
      (`self.K2_DestroyActor` _array_element_2)))
  (`self.K2_DestroyActor`))

(fn `UserConstructionScript`)