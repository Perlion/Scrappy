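; KillZoneBP is a trigger volume that flags the game as won when non-player actors are found inside it.
; Box overlap events maintain the ObjectsInBox array, skipping PlayerBP on entry.
; A check runs at BeginPlay and on a looping ten-second timer, setting HasGameBeenWon on GamemodeBP for each listed actor.
; Its element comparison matches each entry against itself, so it filters nothing by identity.
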(event `self.Box.OnComponentBeginOverlap`
  (params (OverlappedComponent :type "PrimitiveComponent Object Reference") (OtherActor :type "Actor Object Reference") (OtherComp :type "PrimitiveComponent Object Reference") (OtherBodyIndex :type Integer) (bFromSweep :type Boolean) (SweepResult :type "HitResult Structure (by ref)"))
  (cast `/Game/Blueprints/PlayerBP` OtherActor
    (:`CastFailed`
      (`KismetArrayLibrary.Array_Add` (`self.ObjectsInBox`) OtherActor))))

(event `self.Box.OnComponentEndOverlap`
  (params (OverlappedComponent :type "PrimitiveComponent Object Reference") (OtherActor :type "Actor Object Reference") (OtherComp :type "PrimitiveComponent Object Reference") (OtherBodyIndex :type Integer))
  (`KismetArrayLibrary.Array_RemoveItem` (`self.ObjectsInBox`) OtherActor))

(event `self.ReceiveBeginPlay`
  (`KismetSystemLibrary.K2_SetTimerDelegate` (delegate `Itterate Through Array`) 10.0 true)
  (`self.Itterate Through Array`))

(event `Itterate Through Array`
  (bind _objectsinbox (`self.ObjectsInBox`))
  (for (_array_element _array_index) _objectsinbox
    (if (== _array_element (`|GetArrayItem` _objectsinbox _array_index))
      (bind _asgamemode_bp (cast `/Game/Blueprints/GamemodeBP` (`GameplayStatics.GetGameMode`)))
      (set `/Game/Blueprints/GamemodeBP.HasGameBeenWon` true _asgamemode_bp))))

(fn `UserConstructionScript`)