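; Game mode that manages the player HUD, a trash counter and the end-of-game flow.
; BeginPlay shows PlayerHUD, and IncreaseTrash adds a configurable increment to TrashAmount.
; Tick polls HasGameBeenWon, which is not set here, and clears it to fire EndGame once per win.
; EndGame removes all widgets, disables input on the controlled PlayerBP and shows the EndScreen widget.
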(event `self.ReceiveBeginPlay`
  (bind _returnvalue (`|CreateWidget` "/Game/Blueprints/PlayerHUD.PlayerHUD_C" (`GameplayStatics.GetPlayerController` 0)))
  (`UserWidget.AddToViewport` _returnvalue 0))

(event `self.ReceiveTick`
  (params (DeltaSeconds :type "Float (single-precision)"))
  (if (`self.HasGameBeenWon`)
    (set `self.HasGameBeenWon` false)
    (`self.EndGame`)))

(event `EndGame`
  (bind _returnvalue (`GameplayStatics.GetPlayerController` 0))
  (`WidgetLayoutLibrary.RemoveAllWidgets`)
  (bind _asplayer_bp (cast `/Game/Blueprints/PlayerBP` (`Controller.K2_GetPawn` _returnvalue)))
  (`self.DisableInput` _asplayer_bp _returnvalue)
  (bind _returnvalue_2 (`|CreateWidget` "/Game/Blueprints/EndScreen.EndScreen_C" (`GameplayStatics.GetPlayerController` 0)))
  (`UserWidget.AddToViewport` _returnvalue_2 0))

(fn `IncreaseTrash`
  (set `self.TrashAmount` (+ (`self.TrashAmount`) (`self.TrashIncreaseAmount`))))

(fn `UserConstructionScript`)