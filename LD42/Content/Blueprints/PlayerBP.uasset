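; Player pawn that moves along axes from the control yaw cached at BeginPlay and carries trash cubes or ClearBP power-ups.
; One SpawnCube action releases the held object with physics, or when empty-handed spawns a TrashCubeBP if GamemodeBP.TrashAmount is one, otherwise line-traces to grab one.
; Held objects snap to TrashCubeAttach, and releasing a ClearBP also flags it to activate its power-up.
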(event `InputAxis|UP/DOWN`
  (params (AxisValue :type "Float (single-precision)"))
  ;[1 1 1] Movement
  (`self.AddMovementInput` (`KismetMathLibrary.GetForwardVector` (`self.Rotation`)) AxisValue))

(event `InputAxis|Left/Right`
  (params (AxisValue :type "Float (single-precision)"))
  ;[1 1 1] Movement
  (`self.AddMovementInput` (`KismetMathLibrary.GetRightVector` (`self.Rotation`)) AxisValue))

(event `InputAction|SpawnCube`
  (params (Key :type "Key Structure"))
  (bind _staticmesh (`/Game/Blueprints/ClearBP.StaticMesh` (`self.ClearBP`)))
  (bind _staticmesh_2 (`/Game/Blueprints/TrashCubeBP.StaticMesh` (`self.TrashCube`)))
  ;[1 1 1] Cube Movement
  (:`Pressed`
    (if (`self.HasCubeAttached`)
      (if (`self.HasPowerUpAttached`)
        (`PrimitiveComponent.SetSimulatePhysics` _staticmesh true)
        (`PrimitiveComponent.SetEnableGravity` _staticmesh true)
        (set `self.HasPowerUpAttached` false)
        (set `self.HasCubeAttached` false)
        (set `/Game/Blueprints/ClearBP.ActivatePowerup` true (`self.ClearBP`))
        (else
          (`PrimitiveComponent.SetSimulatePhysics` _staticmesh_2 true)
          (`PrimitiveComponent.SetEnableGravity` _staticmesh_2 true)
          (set `self.HasCubeAttached` false)))
      (elif (== (`/Game/Blueprints/GamemodeBP.TrashAmount` (`self.GamemodeBP`)) 1.0)
        (`self.GenerateCubeAndAttach`)
        (else
          (`self.LineTraceToCubeAndAttach`))))))

(event `self.ReceiveBeginPlay`
  (set `self.Rotation` (`KismetMathLibrary.MakeRotator` 0.0 0.0 (.yaw (`self.GetControlRotation`))))
  (bind _asgamemode_bp (cast `/Game/Blueprints/GamemodeBP` (`GameplayStatics.GetGameMode`)))
  (set `self.GamemodeBP` _asgamemode_bp))

(event `LineTraceToCubeAndAttach`
  (bind _staticmesh (`/Game/Blueprints/ClearBP.StaticMesh` (`self.ClearBP`)))
  (bind _staticmesh_2 (`/Game/Blueprints/TrashCubeBP.StaticMesh` (`self.TrashCube`)))
  ;[1 1 1] Line trace to cube + Attach
  (bind _outhit (`KismetSystemLibrary.LineTraceSingle` (`SceneComponent.K2_GetComponentLocation` (`self.LineTraceStart`)) (`SceneComponent.K2_GetComponentLocation` (`self.LineTraceEnd`)) "TraceTypeQuery1"))
  (bind (_bblockinghit _binitialoverlap _time _distance _location _impactpoint _normal _impactnormal _physmat _hitactor) (`GameplayStatics.BreakHitResult` _outhit))
  (bind _astrash_cube_bp (cast `/Game/Blueprints/TrashCubeBP` _hitactor)
    (:`then`
      (set `self.TrashCube` _astrash_cube_bp)
      (`PrimitiveComponent.SetSimulatePhysics` _staticmesh_2 false)
      (`PrimitiveComponent.SetEnableGravity` _staticmesh_2 false)
      (`SceneComponent.K2_AttachToComponent` _staticmesh_2 (`self.TrashCubeAttach`) "None" "SnapToTarget" "KeepRelative" "KeepWorld" true)
      (set `self.HasCubeAttached` true))
    (:`CastFailed`
      (bind _asclear_bp (cast `/Game/Blueprints/ClearBP` _hitactor))
      (set `self.ClearBP` _asclear_bp)
      (`PrimitiveComponent.SetSimulatePhysics` _staticmesh false)
      (`PrimitiveComponent.SetEnableGravity` _staticmesh false)
      (`SceneComponent.K2_AttachToComponent` _staticmesh (`self.TrashCubeAttach`) "None" "SnapToTarget" "KeepRelative" "KeepWorld" true)
      (set `self.HasPowerUpAttached` true)
      (set `self.HasCubeAttached` true))))

(event `self.ReceiveTick`
  (params (DeltaSeconds :type "Float (single-precision)"))
  (if (== (`KismetMathLibrary.MakeRotator` 0.0 0.0 (.yaw (`self.GetControlRotation`))) (`self.Rotation`))
    _))

(event `GenerateCubeAndAttach`
  ;[1 1 1] Spawn Cube + Attach
  (set `self.TrashCubeAmount` (+ (`self.TrashCubeAmount`) 1))
  (set `self.ChangeCube` (+ (`self.ChangeCube`) 1))
  (set `/Game/Blueprints/GamemodeBP.TrashAmount` 0.0 (`self.GamemodeBP`))
  (bind _returnvalue (`|SpawnActorFromClass` "/Game/Blueprints/TrashCubeBP.TrashCubeBP_C" (`KismetMathLibrary.MakeTransform` (`SceneComponent.K2_GetComponentLocation` (`self.TrashCubeAttach`))) "AlwaysSpawn" "OverrideRootScale" null null))
  (set `self.TrashCube` _returnvalue)
  (`self.K2_AttachToComponent` (`self.TrashCube`) (`self.TrashCubeAttach`) "None" "SnapToTarget" "KeepRelative" "KeepRelative" true)
  (set `self.HasCubeAttached` true))

(fn `UserConstructionScript`)