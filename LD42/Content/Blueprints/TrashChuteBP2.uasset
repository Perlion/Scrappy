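; Trash chute actor that periodically spawns random actors once the player has enough trash cubes.
; BeginPlay caches the controlled PlayerBP and starts a short looping timer bound to SpawnStuff.
; Each tick of that timer checks the player's TrashCubeAmount against a fixed threshold without consuming it.
; When met, it spawns a random class from the TireFrame array at the Scene component's location, ignoring collisions.
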(event `self.ReceiveBeginPlay`
  (bind _asplayer_bp (cast `/Game/Blueprints/PlayerBP` (`Controller.K2_GetPawn` (`GameplayStatics.GetPlayerController` 0))))
  (set `self.PlayerBP` _asplayer_bp)
  (`KismetSystemLibrary.K2_SetTimerDelegate` (delegate `SpawnStuff`) 0.7 true))

(event `SpawnStuff`
  (bind _tireframe (`self.TireFrame`))
  (bind _returnvalue_location (`KismetMathLibrary.BreakTransform` (`SceneComponent.K2_GetComponentToWorld` (`self.Scene`))))
  (if (>= (`/Game/Blueprints/PlayerBP.TrashCubeAmount` (`self.PlayerBP`)) 5)
    (`|SpawnActorFromClass` (`|GetArrayItem` _tireframe (`KismetMathLibrary.RandomInteger` (`KismetArrayLibrary.Array_Length` _tireframe))) (`KismetMathLibrary.MakeTransform` _returnvalue_location) "AlwaysSpawn" "OverrideRootScale" null null)))

(fn `UserConstructionScript`)